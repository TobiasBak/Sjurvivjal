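; Base AI enemy character that handles hit reactions, melee attacks on the player and difficulty scaling.
; TakeDamage runs parent logic, then, if still alive, plays a hit animation while flagging IsTakingDamage on the blackboard.
; Attack plays a montage, damages the player halfway through if within AttackDistance, and signals OnAttackEnd afterwards.
; UpdateDifficulty multiplies base health and damage in place, so repeated calls compound, and refills current health.
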(event `/Game/Engine/BPI/BPI_Attack.TakeDamage`
  (params (Damage :type "Float (double-precision)"))
  ; Take Damage Animation
  (`parent.TakeDamage` Damage)
  (bind _alive (`self.IsAlive`))
  (if _alive
    (`BlackboardComponent.SetValueAsBool` (`AIBlueprintHelperLibrary.GetBlackboard` null) (`KismetMathLibrary.SelectName` "IsTakingDamage" "None" true) true)
    (`SkeletalMeshComponent.PlayAnimation` (`self.Mesh`) "/Game/Characters/Mannequins/Anims/Rifle/HitReact/MM_HitReact_Front_Hvy_01.MM_HitReact_Front_Hvy_01" false)
    (`KismetSystemLibrary.Delay` 0.7)
    (`SkeletalMeshComponent.SetAnimationMode` (`self.Mesh`) "AnimationBlueprint" false)
    (`BlackboardComponent.SetValueAsBool` (`AIBlueprintHelperLibrary.GetBlackboard` null) (`KismetMathLibrary.SelectName` "IsTakingDamage" "None" true) false)))

(event `Attack`
  (bind _returnvalue (`GameplayStatics.GetPlayerCharacter` 0))
  ; Attack
  (bind _returnvalue_2 (`self.PlayAnimMontage` "/Game/Characters/Mannequins/Anims/Unarmed/Attack/Enemy_attack.Enemy_attack"))
  (bind _returnvalue_3 (/ _returnvalue_2 2.0))
  (`KismetSystemLibrary.Delay` _returnvalue_3)
  (if (<= (`KismetMathLibrary.Vector_Distance` (`self.K2_GetActorLocation` _returnvalue) (`self.K2_GetActorLocation` self)) (`self.AttackDistance`))
    (message `/Game/Engine/BPI/BPI_Attack.TakeDamage` _returnvalue (`self.BaseDamage`)))
  (`KismetSystemLibrary.Delay` _returnvalue_3)
  (`self.OnAttackEnd`))

(event `self.UpdateDifficulty`
  (params (Difficulty :type "Float (single-precision)"))
  ; Basic Difficulty Update
  (bind _output_get (set `self.Difficulty` Difficulty))
  (bind _output_get_2 (set `self.BaseHealth` (* _output_get (`self.BaseHealth`))))
  (set `self.CurrentHealth` _output_get_2)
  (set `self.BaseDamage` (* (`self.Difficulty`) (`self.BaseDamage`))))

(fn `UserConstructionScript`
  (`parent.UserConstructionScript`))